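; NinjaController tracks the player's coin total and handles spawning and possessing the Ninja character.
; Its construction script loads the saved total from the "Coin" save slot.
; AddCoin raises that total and a per-level tally, checked against the level name cached on BeginPlay.
; SpawnNinja spawns a Ninja at the first PlayerStart found, possesses it, and deducts the level tally, rolling back coins gained on that level.
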(event `self.ReceiveBeginPlay`
  (bind _returnvalue (`GameplayStatics.GetCurrentLevelName` true))
  (set `self.LevelName` _returnvalue))

(fn `AddCoin`
  (params (CoinAdded :type Integer))
  (set `self.Coins` (+ CoinAdded (`self.Coins`)))
  (bind _returnvalue (`GameplayStatics.GetCurrentLevelName` true))
  (if (== (`self.LevelName`) _returnvalue)
    (set `self.CoinAddedOnLevel` (+ (`local.CoinAdded`) (`self.CoinAddedOnLevel`)))))

(fn `SpawnNinja`
  (bind _outactors (`GameplayStatics.GetAllActorsOfClass` "/Script/Engine.PlayerStart"))
  (if (> (`KismetArrayLibrary.Array_Length` _outactors) 0)
    (bind _returnvalue (`|SpawnActorFromClass` "/Game/Blueprints/Character/Ninja.Ninja_C" (`self.GetTransform` (`|GetArrayItem` _outactors)) "Undefined" "OverrideRootScale" null null))
    (`self.Possess` (`GameplayStatics.GetPlayerController` 0) _returnvalue)
    (set `self.Coins` (- (`self.Coins`) (`self.CoinAddedOnLevel`)))
    (set `self.CoinAddedOnLevel` 0)))

(fn `UserConstructionScript`
  (set `self.CoinAddedOnLevel` 0)
  (bind _returnvalue (`GameplayStatics.DoesSaveGameExist` "Coin"))
  (if _returnvalue
    (bind _returnvalue_2 (`GameplayStatics.LoadGameFromSlot` "Coin"))
    (bind _ascoin_save (cast `/Game/Blueprints/CoinSave` _returnvalue_2))
    (bind _output_get (set `self.CoinSv` _ascoin_save))
    (set `self.Coins` (`/Game/Blueprints/CoinSave.Coin` _output_get))))