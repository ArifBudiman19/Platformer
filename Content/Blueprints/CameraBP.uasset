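; Camera actor that follows the player between MinX and MaxX markers at a fixed rotation.
; Each tick MakeFollow eases the camera toward the player's X/Y, or to MinX below that bound, keeping MinX's height and ignoring TargetZ.
; Past MaxX it stops updating, as that follow call is disconnected.
; Without a valid player, it takes the view target, re-armed by a delay, and eases back to MinX.
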(event `self.ReceiveBeginPlay`
  (set `self.playerCharacter` (`GameplayStatics.GetPlayerCharacter` 0)))

(event `self.ReceiveTick`
  (params (DeltaSeconds :type "Float (single-precision)"))
  (bind _returnvalue_x (`KismetMathLibrary.BreakVector` (`self.K2_GetActorLocation` (`self.playerCharacter`))))
  (bind _returnvalue (`self.K2_GetActorLocation` (`self.playerCharacter`)))
  (bind _returnvalue_x_2 (`KismetMathLibrary.BreakVector` (`SceneComponent.K2_GetComponentLocation` (`self.MinX`))))
  (bind _returnvalue_x_3 (`KismetMathLibrary.BreakVector` (`self.K2_GetActorLocation` (`self.playerCharacter`))))
  (bind (_returnvalue_x_4 _returnvalue_y _returnvalue_z) (`KismetMathLibrary.BreakVector` (`self.K2_GetActorLocation` (`self.playerCharacter`))))
  (bind _returnvalue_x_5 (`KismetMathLibrary.BreakVector` (`SceneComponent.K2_GetComponentLocation` (`self.MaxX`))))
  (set `self.DeltaTime` DeltaSeconds)
  (`|ExecutionSequence`
    (:`then_0`
      (`/Engine/EditorBlueprintResources/StandardMacros.IsValid` (`self.playerCharacter`)
        (:`Is Not Valid`
          (set `self.playerCharacter` (`GameplayStatics.GetPlayerCharacter` 0)))))
    (:`then_1`
      (`/Engine/EditorBlueprintResources/StandardMacros.IsValid` (`self.playerCharacter`)
        (:`Is Valid`
          (if (< _returnvalue_x_3 _returnvalue_x_2)
            (`self.MakeFollow` (`SceneComponent.K2_GetComponentLocation` (`self.MinX`)) (`self.DeltaTime`) _returnvalue_z 10.0)
            (elif (not (> _returnvalue_x _returnvalue_x_5))
              (`self.MakeFollow` _returnvalue (`self.DeltaTime`) (.z _returnvalue) 10.0))))
        (:`Is Not Valid`
          (`|ExecutionSequence`
            (:`then_0`
              (`/Engine/EditorBlueprintResources/StandardMacros.DoOnce` false :!label _label
                (:`Completed`
                  (`PlayerController.SetViewTargetWithBlend` (`GameplayStatics.GetPlayerController` 0) self 0.0 "VTBlend_Linear" 0.0 false)
                  (`KismetSystemLibrary.RetriggerableDelay` 10.0)
                  (goto _label :!via `Reset`))))
            (:`then_1`
              (`SceneComponent.K2_SetWorldLocationAndRotation` (`self.CameraComponent`) (`KismetMathLibrary.VInterpTo` (`SceneComponent.K2_GetComponentLocation` (`self.CameraComponent`)) (`SceneComponent.K2_GetComponentLocation` (`self.MinX`)) (`self.DeltaTime`) 3.0) (struct :`Yaw` -90.0) false true))))))))

(fn `MakeFollow`
  (params (TargetLocation :type "Vector Structure") (DeltaTime :type "Float (double-precision)") (Target_Z :type "Float (double-precision)") (InterpSpeed :type "Float (double-precision)"))
  (bind _cameracomponent (`self.CameraComponent`))
  (bind (_returnvalue_x _returnvalue_y _returnvalue_z) (`KismetMathLibrary.BreakVector` (`SceneComponent.K2_GetComponentLocation` (`self.MinX`))))
  (`SceneComponent.K2_SetWorldLocationAndRotation` _cameracomponent (`KismetMathLibrary.VInterpTo` (`SceneComponent.K2_GetComponentLocation` _cameracomponent) (`KismetMathLibrary.MakeVector` (.x TargetLocation) (.y TargetLocation) _returnvalue_z) DeltaTime InterpSpeed) (struct :`Yaw` -90.0) false false))

(fn `UserConstructionScript`)