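; Level-exit trigger that saves the player's coins and loads the next level when the Ninja walks into it.
; On Box overlap by a Ninja, it creates a fresh CoinSave object and copies in the coin count from the NinjaController of player 0.
; It saves that object to the Coin slot, then opens the level named by TargetLevel.
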(event `self.Box.OnComponentBeginOverlap`
  (params (OverlappedComponent :type "PrimitiveComponent Object Reference") (OtherActor :type "Actor Object Reference") (OtherComp :type "PrimitiveComponent Object Reference") (OtherBodyIndex :type Integer) (bFromSweep :type Boolean) (SweepResult :type "HitResult Structure (by ref)"))
  (cast `/Game/Blueprints/Character/Ninja` OtherActor)
  (bind _returnvalue (`GameplayStatics.CreateSaveGameObject` "/Game/Blueprints/CoinSave.CoinSave_C"))
  (bind _ascoin_save (cast `/Game/Blueprints/CoinSave` _returnvalue))
  (set `self.CoinSave` _ascoin_save)
  (bind _asninja_controller (cast `/Game/Blueprints/Controller/NinjaController` (`GameplayStatics.GetPlayerController` 0)))
  (set `/Game/Blueprints/CoinSave.Coin` (`/Game/Blueprints/Controller/NinjaController.Coins` _asninja_controller) (`self.CoinSave`))
  (`GameplayStatics.SaveGameToSlot` (`self.CoinSave`) "Coin")
  (`GameplayStatics.OpenLevel` (`self.TargetLevel`)))

(fn `UserConstructionScript`)