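; ProceduralBG is a Blueprint actor that builds a horizontal strip of Paper2D background sprites.
; Its construction script assigns the Background sprite to the BG component, then adds Length minus one extra sprite components at fixed intervals along X.
; The added components have collision disabled, and the script does not explicitly assign Background to them.
; The event graph holds only disabled placeholder events, so it adds no runtime logic.
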(fn `UserConstructionScript`
  (`PaperSpriteComponent.SetSprite` (`self.BG`) (`self.Background`))
  (if (> (`self.Length`) 1)
    (for _index (range 2 (+ (`self.Length`) 1))
      (bind _returnvalue (`AddComponent|NODE_AddPaperSpriteComponent-0` :`RelativeTransform` (`KismetMathLibrary.MakeTransform` (`KismetMathLibrary.MakeVector` (* (- _index 1) 1000.0)))))
      (`PrimitiveComponent.SetCollisionEnabled` _returnvalue "NoCollision"))))