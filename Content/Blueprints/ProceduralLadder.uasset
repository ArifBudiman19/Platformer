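; Procedural ladder Blueprint that Ninja characters can climb, with its height set by a Length variable.
; The construction script stacks Paper2D sprite components at fixed vertical spacing, randomly picking one of two add-component branches per segment, then centers and sizes the Box to cover the stack.
; Box overlaps call TriggerClimb on the Ninja, passing the ladder on entry and nothing on exit.
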(event `self.Box.OnComponentBeginOverlap`
  (params (OverlappedComponent :type "PrimitiveComponent Object Reference") (OtherActor :type "Actor Object Reference") (OtherComp :type "PrimitiveComponent Object Reference") (OtherBodyIndex :type Integer) (bFromSweep :type Boolean) (SweepResult :type "HitResult Structure (by ref)"))
  (bind _asninja (cast `/Game/Blueprints/Character/Ninja` OtherActor))
  (`/Game/Blueprints/Character/Ninja.TriggerClimb` _asninja self))

(event `self.Box.OnComponentEndOverlap`
  (params (OverlappedComponent :type "PrimitiveComponent Object Reference") (OtherActor :type "Actor Object Reference") (OtherComp :type "PrimitiveComponent Object Reference") (OtherBodyIndex :type Integer))
  (bind _asninja (cast `/Game/Blueprints/Character/Ninja` OtherActor))
  (`/Game/Blueprints/Character/Ninja.TriggerClimb` _asninja null))

(fn `UserConstructionScript`
  (`|ExecutionSequence`
    (:`then_0`
      (for _index (range 1 (+ (`self.Length`) 1))
        (if (`KismetMathLibrary.RandomBool`)
          (bind _returnvalue (`KismetMathLibrary.MakeVector` 0.0 0.0 (* (- _index 1) 32.0)))
          (`AddComponent|NODE_AddPaperSpriteComponent-1` :`RelativeTransform` (`KismetMathLibrary.MakeTransform` _returnvalue))
          (else
            (`AddComponent|NODE_AddPaperSpriteComponent-2` :`RelativeTransform` (`KismetMathLibrary.MakeTransform` _returnvalue))))))
    (:`then_1`
      (`SceneComponent.K2_SetRelativeLocation` (`self.Box`) (`KismetMathLibrary.MakeVector` 0.0 0.0 (* (- (`self.Length`) 1) 16.0)) false false)
      (`BoxComponent.SetBoxExtent` (`self.Box`) (`KismetMathLibrary.MakeVector` 16.0 32.0 (* (`self.Length`) 16.0)) true))))