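; Collectible coin actor that the player's Ninja picks up by overlapping its sphere.
; On overlap with a Ninja, it adds one coin through the first player's NinjaController and then hides itself.
; Hiding disables collision and the billboard's visibility rather than destroying the actor, and AppearCoin restores both so the coin can be reused.
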(event `self.Sphere.OnComponentBeginOverlap`
  (params (OverlappedComponent :type "PrimitiveComponent Object Reference") (OtherActor :type "Actor Object Reference") (OtherComp :type "PrimitiveComponent Object Reference") (OtherBodyIndex :type Integer) (bFromSweep :type Boolean) (SweepResult :type "HitResult Structure (by ref)"))
  (cast `/Game/Blueprints/Character/Ninja` OtherActor)
  (bind _asninja_controller (cast `/Game/Blueprints/Controller/NinjaController` (`GameplayStatics.GetPlayerController` 0)))
  (`/Game/Blueprints/Controller/NinjaController.AddCoin` _asninja_controller 1)
  (`self.HideCoin`))

(event `HideCoin`
  (`self.SetActorEnableCollision` false)
  (`SceneComponent.SetVisibility` (`self.Billboard`) false true))

(event `AppearCoin`
  (`self.SetActorEnableCollision` true)
  (`SceneComponent.SetVisibility` (`self.Billboard`) true true))

(fn `UserConstructionScript`)