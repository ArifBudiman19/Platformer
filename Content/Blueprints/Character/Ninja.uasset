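; Paper2D side-scrolling ninja player character that runs, double-jumps, glides, slides, climbs ladders, throws kunai and slashes.
; Input events set state flags and tune gravity or friction: held jump glides, slash box-traces for damage.
; Tick-driven AnimationUpdate derives an enum state, selects flipbooks, mirrors the sprite and locks Y; Tick also shrinks the capsule while sliding.
; TriggerClimb toggles custom movement, damage handles death, and Respawn possesses a new ninja at a PlayerStart.
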(event `self.ReceiveTick`
  (params (DeltaSeconds :type "Float (single-precision)"))
  (`|ExecutionSequence`
    (:`then_0`
      (`self.AnimationUpdate`))
    (:`then_1`
      (if (not (`self.isGliding`))
        (set `CharacterMovementComponent.GravityScale` 1.0 (`self.CharacterMovement`))))
    (:`then_2`
      (if (not (`self.isSliding`))
        (set `CharacterMovementComponent.GroundFriction` 8.0 (`self.CharacterMovement`)))
      (`CapsuleComponent.SetCapsuleHalfHeight` (`self.CapsuleComponent`) (`KismetMathLibrary.FInterpTo_Constant` (`CapsuleComponent.CapsuleHalfHeight` (`self.CapsuleComponent`)) (select `bool` (`self.isSliding`) :`false` 40.0 :`true` 20.0 :!type "Float (single-precision)") (`GameplayStatics.GetWorldDeltaSeconds`) 20.0) true))))

(event `self.K2_OnMovementModeChanged`
  (params (PrevMovementMode :type "EMovementMode Enum" :default "MOVE_None") (NewMovementMode :type "EMovementMode Enum" :default "MOVE_None") (PrevCustomMode :type Byte) (NewCustomMode :type Byte))
  (set `self.CurrentCustomMovement` NewCustomMode))

(event `self.K2_UpdateCustomMovement`
  (params (DeltaTime :type "Float (single-precision)"))
  (if (== (`self.CurrentCustomMovement`) (enumliteral `/Game/Blueprints/NinjaState` "NewEnumerator1"))
    (`self.K2_SetActorLocation` (`self.CalcModeClimb`) true)))

(event `InputAxis|MoveUp`
  (params (AxisValue :type "Float (single-precision)"))
  (if (and (not (`self.isDead`)) (`KismetSystemLibrary.IsValid` (`self.Ladder`)))
    (`self.AddMovementInput` (0.0 0.0 1.0) AxisValue)))

(event `InputAxis|MoveRight`
  (params (AxisValue :type "Float (single-precision)"))
  (if (not (`self.isDead`))
    (`/Engine/EditorBlueprintResources/StandardMacros.CompareFloat` AxisValue
      (:`>`
        (set `self.isFacingRight` true))
      (:`<`
        (set `self.isFacingRight` false)))
    (`self.AddMovementInput` (1.0 0.0 0.0) (`self.GetInputAxisValue`))))

(event `InputAction|Slide`
  (params (Key :type "Key Structure"))
  (:`Pressed`
    (if (not (or (`self.isSliding`) (not (`NavMovementComponent.IsMovingOnGround` (`self.CharacterMovement`)))))
      (set `CharacterMovementComponent.GroundFriction` 0.001 (`self.CharacterMovement`))
      (set `self.isSliding` true)
      (`self.LaunchCharacter` (`KismetMathLibrary.MakeVector` (* (`self.CalcScaleX`) (`self.slideForce`))))
      (`KismetSystemLibrary.RetriggerableDelay` 0.25)
      (if (`self.isSliding`)
        (set `self.isSliding` false)
        (set `CharacterMovementComponent.GroundFriction` 8.0 (`self.CharacterMovement`))))))

(event `InputAction|Jump`
  (params (Key :type "Key Structure"))
  (:`Pressed`
    (if (not (`self.isDead`))
      (`|ExecutionSequence`
        (:`then_0`
          (if (< (`self.JumpCurrentCount`) (`self.JumpMaxCount`))
            (`self.Jump`)
            (if (not (or (`self.isFirstJump`) (!= (`self.JumpCurrentCount`) 0) (`self.isGliding`)))
              (set `self.isFirstJump` true)
              (`PaperFlipbookComponent.SetFlipbook` (`self.Sprite`) "/Game/Flipbooks/Ninja/NInjaJumpFB.NInjaJumpFB")
              (`KismetSystemLibrary.RetriggerableDelay` 0.3)
              (set `self.isFirstJump` false))))
        (:`then_1`
          (goto _label :!via `Open`))
        (:`then_2`
          (`KismetSystemLibrary.RetriggerableDelay` 0.5)
          (`/Engine/EditorBlueprintResources/StandardMacros.Gate` true :!label _label
            (:`Exit`
              (set `self.isGliding` true)
              (if (`NavMovementComponent.IsFalling` (`self.CharacterMovement`))
                (`MovementComponent.StopMovementImmediately` (`self.CharacterMovement`))
                (set `CharacterMovementComponent.GravityScale` 0.03 (`self.CharacterMovement`)))))))))
  (:`Released`
    (`self.StopJumping`)
    (set `self.isGliding` false)
    (set `CharacterMovementComponent.GravityScale` 1.0 (`self.CharacterMovement`))
    (goto _label :!via `Close`)))

(event `self.OnLanded`
  (params (Hit :type "HitResult Structure (by ref)"))
  (set `CharacterMovementComponent.GravityScale` 1.0 (`self.CharacterMovement`)))

(event `InputAction|Throw`
  (params (Key :type "Key Structure"))
  (bind (_returnvalue_location _returnvalue_rotation) (`KismetMathLibrary.BreakTransform` (`SceneComponent.K2_GetComponentToWorld` (`self.ThrowOffset`))))
  (bind _returnvalue (`NavMovementComponent.IsFalling` (`self.CharacterMovement`)))
  (:`Pressed`
    (if (and (not (`self.isDead`)) (not (`self.onThrowing`)))
      (set `self.isAttacking` true)
      (set `self.onThrowing` true)
      (`MovementComponent.StopMovementImmediately` (`self.CharacterMovement`))
      (`PaperFlipbookComponent.SetFlipbook` (`self.Sprite`) (select `bool` _returnvalue :`false` "/Game/Flipbooks/Ninja/NinjaThrowFB.NinjaThrowFB" :`true` "/Game/Flipbooks/Ninja/NInjaJumpThrowFB.NInjaJumpThrowFB" :!type "PaperFlipbook Object Reference"))
      (set `self.State` (select `bool` _returnvalue :`false` "NewEnumerator12" :`true` "NewEnumerator9" :!type "/Game/Blueprints/NinjaState Enum"))
      (`KismetSystemLibrary.RetriggerableDelay` 0.15)
      (`|SpawnActorFromClass` "/Game/Blueprints/KunaiBP.KunaiBP_C" (`KismetMathLibrary.MakeTransform` _returnvalue_location _returnvalue_rotation) "Undefined" "OverrideRootScale" self null)
      (set `self.isAttacking` false)
      (set `self.State` (select `bool` (`NavMovementComponent.IsFalling` (`self.CharacterMovement`)) :`false` "NewEnumerator5" :`true` (select `bool` (`self.isGliding`) :`false` "NewEnumerator8" :`true` "NewEnumerator4" :!type "/Game/Blueprints/NinjaState Enum")))
      (`KismetSystemLibrary.Delay` 0.02)
      (set `self.onThrowing` false))))

(event `InputAction|Slash`
  (params (Key :type "Key Structure"))
  (bind _returnvalue (`NavMovementComponent.IsFalling` (`self.CharacterMovement`)))
  (:`Pressed`
    (if (and (not (`self.isDead`)) (not (`self.onSlashing`)))
      (set `self.isAttacking` true)
      (set `self.onSlashing` true)
      (`MovementComponent.StopMovementImmediately` (`self.CharacterMovement`))
      (`PaperFlipbookComponent.SetFlipbook` (`self.Sprite`) (select `bool` _returnvalue :`false` "/Game/Flipbooks/Ninja/NinjaAttackFB.NinjaAttackFB" :`true` "/Game/Flipbooks/Ninja/NInjaJumpAttackFB.NInjaJumpAttackFB" :!type "PaperFlipbook Object Reference"))
      (set `self.State` (select `bool` _returnvalue :`false` "NewEnumerator0" :`true` "NewEnumerator6" :!type "/Game/Blueprints/NinjaState Enum"))
      (bind (_outhit _returnvalue_2) (`KismetSystemLibrary.BoxTraceSingle` (- (`self.K2_GetActorLocation`) (0.0 0.0 9.0)) (`SceneComponent.K2_GetComponentLocation` (`self.SlashOffset`)) (0.0 32.0 32.0) (struct) "TraceTypeQuery2"))
      (`|ExecutionSequence`
        (:`then_0`
          (if _returnvalue_2
            (`GameplayStatics.ApplyDamage` (`.HitActor` (`GameplayStatics.BreakHitResult` _outhit)) 1.0 null self)))
        (:`then_1`
          (`KismetSystemLibrary.RetriggerableDelay` 0.3)
          (set `self.isAttacking` false)
          (set `self.State` (select `bool` false :`false` "NewEnumerator5" :`true` (select `bool` (`self.isGliding`) :`false` "NewEnumerator8" :`true` "NewEnumerator4" :!type "/Game/Blueprints/NinjaState Enum")))
          (set `self.onSlashing` false))))))

(event `self.ReceiveAnyDamage`
  (params (Damage :type "Float (single-precision)") (DamageType :type "DamageType Object Reference") (InstigatedBy :type "Controller Object Reference") (DamageCauser :type "Actor Object Reference"))
  (set `self.Health` (- (`self.Health`) Damage))
  (if (<= (`self.Health`) 0.0)
    (set `self.isDead` true)
    (set `self.State` "NewEnumerator3")
    (`PaperFlipbookComponent.SetFlipbook` (`self.Sprite`) "/Game/Flipbooks/Ninja/NinjaDeadFB.NinjaDeadFB")
    (set `CharacterMovementComponent.GravityScale` 0.0 (`self.CharacterMovement`))
    (`PrimitiveComponent.SetCollisionEnabled` (`self.CapsuleComponent`) "NoCollision")
    (`KismetSystemLibrary.RetriggerableDelay` 0.6)
    (`self.K2_DestroyActor`)))

(event `Respawn`
  (bind _outactors (`GameplayStatics.GetAllActorsOfClass` "/Script/Engine.PlayerStart"))
  (if (> (`KismetArrayLibrary.Array_Length` _outactors) 0)
    (bind _returnvalue (`|SpawnActorFromClass` "Ninja_C" (`self.GetTransform` (`|GetArrayItem` _outactors)) "Undefined" "OverrideRootScale" null null))
    (`Controller.Possess` (`GameplayStatics.GetPlayerController` 0) _returnvalue)))

(fn `AnimationUpdate`
  (bind (_returnvalue_x _returnvalue_y _returnvalue_z) (`KismetMathLibrary.BreakVector` (`self.K2_GetActorLocation`)))
  (bind _isfacingright (`self.isFacingRight`))
  (bind _returnvalue (select `bool` _isfacingright :`false` 180.0 :!type "Float (single-precision)"))
  (bind (_relativescale3d_x _relativescale3d_y _relativescale3d_z) (`KismetMathLibrary.BreakVector` (`SceneComponent.RelativeScale3D` (`self.Sprite`))))
  (`|ExecutionSequence`
    (:`then_0`
      (`SceneComponent.K2_SetRelativeLocation` (`self.Sprite`) (`KismetMathLibrary.MakeVector` (* (select `/Game/Blueprints/NinjaState` (`self.State`) :`NewEnumerator0` 24.0 :`NewEnumerator3` 24.0 :`NewEnumerator6` 24.0 :!type "Float (single-precision)") (`self.CalcScaleX`)) 0.0 (select `/Game/Blueprints/NinjaState` (`self.State`) :`NewEnumerator0` -13.0 :`NewEnumerator1` -9.0 :`NewEnumerator2` -9.0 :`NewEnumerator3` -9.0 :`NewEnumerator4` -9.0 :`NewEnumerator5` -9.0 :`NewEnumerator6` -9.0 :`NewEnumerator7` -9.0 :`NewEnumerator8` -9.0 :`NewEnumerator9` -9.0 :`NewEnumerator10` -9.0 :`NewEnumerator11` -9.0 :`NewEnumerator12` -9.0 :!type "Float (single-precision)")) false false)
      (`self.K2_SetActorLocation` (`KismetMathLibrary.MakeVector` _returnvalue_x (`self.initY`) _returnvalue_z) false true))
    (:`then_1`
      (`SceneComponent.SetRelativeScale3D` (`self.Sprite`) (`KismetMathLibrary.MakeVector` (* (`self.scaleX`) (`self.CalcScaleX`)) _relativescale3d_y _relativescale3d_z))
      (`SceneComponent.K2_SetRelativeLocationAndRotation` (`self.ThrowOffset`) (select `bool` false :`false` (200.0 0.0 0.0) :`true` (200.0 0.0 -90.0) :!type "Vector Structure") (select `bool` (`NavMovementComponent.IsFalling` (`self.CharacterMovement`)) :`false` (`KismetMathLibrary.MakeRotator` 0.0 (select `bool` _isfacingright :`false` 90.0 :`true` -90.0 :!type "Float (single-precision)") _returnvalue) :`true` (`KismetMathLibrary.MakeRotator` 0.0 (select `bool` _isfacingright :`false` 106.0 :`true` -106.0 :!type "Float (single-precision)") _returnvalue) :!type "Rotator Structure") false false))
    (:`then_2`
      (if (and (not (`self.isDead`)) (not (`self.isAttacking`)) (not (`self.isFirstJump`)))
        (set `self.State` (select `bool` (`self.isClimbing`) :`false` (select `bool` (`NavMovementComponent.IsMovingOnGround` (`self.CharacterMovement`)) :`false` (select `bool` (`self.isGliding`) :`false` "NewEnumerator8" :`true` "NewEnumerator4" :!type "/Game/Blueprints/NinjaState Enum") :`true` (select `bool` (!= (`MovementComponent.Velocity` (`self.CharacterMovement`)) (0.0 0.0 0.0)) :`false` "NewEnumerator5" :`true` (select `bool` (`self.isSliding`) :`false` "NewEnumerator11" :`true` "NewEnumerator10" :!type "/Game/Blueprints/NinjaState Enum"))) :`true` (select `bool` (!= (`MovementComponent.Velocity` (`self.CharacterMovement`)) (0.0 0.0 0.0)) :`false` "NewEnumerator5" :`true` "NewEnumerator1" :!type "/Game/Blueprints/NinjaState Enum")))
        (`PaperFlipbookComponent.SetFlipbook` (`self.Sprite`) (select `/Game/Blueprints/NinjaState` (`self.State`) :`NewEnumerator0` "/Game/Flipbooks/Ninja/NinjaAttackFB.NinjaAttackFB" :`NewEnumerator1` "/Game/Flipbooks/Ninja/NinjaClimbFB.NinjaClimbFB" :`NewEnumerator2` "/Game/Flipbooks/Ninja/NinjaClimbIdleFB.NinjaClimbIdleFB" :`NewEnumerator3` "/Game/Flipbooks/Ninja/NinjaDeadFB.NinjaDeadFB" :`NewEnumerator4` "/Game/Flipbooks/Ninja/NinjaGlideFB.NinjaGlideFB" :`NewEnumerator5` "/Game/Flipbooks/Ninja/NInjaIdleFB.NInjaIdleFB" :`NewEnumerator6` "/Game/Flipbooks/Ninja/NInjaJumpAttackFB.NInjaJumpAttackFB" :`NewEnumerator7` "/Game/Flipbooks/Ninja/NInjaJumpFB.NInjaJumpFB" :`NewEnumerator8` "/Game/Flipbooks/Ninja/NInjaJumpEndFB.NInjaJumpEndFB" :`NewEnumerator9` "/Game/Flipbooks/Ninja/NinjaThrowFB.NinjaThrowFB" :`NewEnumerator10` "/Game/Flipbooks/Ninja/NinjaSlideFB.NinjaSlideFB" :`NewEnumerator11` "/Game/Flipbooks/Ninja/NinjaRunFB.NinjaRunFB" :`NewEnumerator12` "/Game/Flipbooks/Ninja/NinjaThrowFB.NinjaThrowFB" :!type "PaperFlipbook Object Reference"))))))

(fn `TriggerClimb`
  (params (Ladder :type "/Game/Blueprints/ProceduralLadder Object Reference"))
  (bind _output_get (set `self.Ladder` Ladder))
  (`/Engine/EditorBlueprintResources/StandardMacros.IsValid` _output_get
    (:`Is Valid`
      (`CharacterMovementComponent.SetMovementMode` (`self.CharacterMovement`) "MOVE_Custom" (enumliteral `/Game/Blueprints/NinjaState` "NewEnumerator1")))
    (:`Is Not Valid`
      (`CharacterMovementComponent.SetMovementMode` (`self.CharacterMovement`) "MOVE_Walking" 0))))

(fn `UserConstructionScript`
  (bind (_returnvalue_x _returnvalue_y) (`KismetMathLibrary.BreakVector` (`self.K2_GetActorLocation`)))
  (bind _relativescale3d_x (`KismetMathLibrary.BreakVector` (`SceneComponent.RelativeScale3D` (`self.Sprite`))))
  (set `self.initY` _returnvalue_y)
  (set `self.scaleX` _relativescale3d_x)
  (set `self.JumpMaxCount` 2))