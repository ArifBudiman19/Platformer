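; Sword-wielding ninja enemy for a 2D Paper2D side-scroller that patrols left and right on a locked Y axis.
; Each Tick, traces flip it at ledges, other ninjas or sprite obstacles, and an optional distance budget also turns it around.
; Spotting the player triggers a randomly delayed box-trace attack.
; Damage briefly stops movement with a random hurt flipbook and destroys it at zero health.
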(event `AIControl`
  (if (not (or (`self.onDamage`) (`self.onAttack`)))
    (`|ExecutionSequence`
      (:`then_0`
        (`self.Move`))
      (:`then_1`
        (if (<= (`self.distanceToFlip`) 0.0)
          (`/Engine/EditorBlueprintResources/StandardMacros.DoOnce` false :!label _label
            (:`Completed`
              (`self.Flip`)
              (`KismetSystemLibrary.RetriggerableDelay` (`KismetMathLibrary.RandomFloatInRange` 0.3 0.6))
              (goto _label :!via `Reset`))))))))

(event `AIDetection`
  (`|ExecutionSequence`
    (:`then_0`
      (bind _returnvalue (`self.HasGroundOnFront`))
      (if (not _returnvalue)
        (`/Engine/EditorBlueprintResources/StandardMacros.DoOnce` false :!label _label_2
          (:`Completed`
            (`self.Flip`)
            (`KismetSystemLibrary.Delay` 0.6)
            (goto _label_2 :!via `Reset`)))))
    (:`then_1`
      (bind _return_value (`self.HasEnemyOnFront`))
      (if (and _return_value (not (`self.onAttack`)))
        (`/Engine/EditorBlueprintResources/StandardMacros.DoOnce` false :!label _label_3
          (:`Completed`
            (`KismetSystemLibrary.RetriggerableDelay` (`KismetMathLibrary.RandomFloatInRange` 0.2 0.7))
            (set `self.onAttack` true)
            (`self.Attack`)
            (`PaperFlipbookComponent.SetFlipbook` (`self.Sprite`) "/Game/Flipbooks/NinjaSword/SNinja_Atk.SNinja_Atk")
            (`KismetSystemLibrary.RetriggerableDelay` 0.4)
            (set `self.onAttack` false)
            (`KismetSystemLibrary.RetriggerableDelay` 0.01)
            (goto _label_3 :!via `Reset`)))))
    (:`then_2`
      (bind _returnvalue_2 (`self.HasObstaclesOnFront`))
      (if _returnvalue_2
        (`/Engine/EditorBlueprintResources/StandardMacros.DoOnce` false :!label _label_4
          (:`Completed`
            (`self.Flip`)
            (`KismetSystemLibrary.Delay` 0.6)
            (goto _label_4 :!via `Reset`)))))))

(event `self.ReceiveTick`
  (params (DeltaSeconds :type "Float (single-precision)"))
  (bind (_returnvalue_x _returnvalue_y _returnvalue_z) (`KismetMathLibrary.BreakVector` (`self.K2_GetActorLocation`)))
  (set `self.deltaTime` DeltaSeconds)
  (if (not (`self.isDead`))
    (`|ExecutionSequence`
      (:`then_0`
        (`self.AIDetection`))
      (:`then_1`
        (`self.K2_SetActorLocation` (`KismetMathLibrary.MakeVector` _returnvalue_x (`self.initY`) _returnvalue_z) false true)
        (`self.AIControl`)))))

(event `self.ReceiveBeginPlay`
  (if (`KismetMathLibrary.RandomBool`)
    (`self.Flip`)))

(event `self.ReceiveAnyDamage`
  (params (Damage :type "Float (single-precision)") (DamageType :type "DamageType Object Reference") (InstigatedBy :type "Controller Object Reference") (DamageCauser :type "Actor Object Reference"))
  (set `self.health` (- (`self.health`) Damage))
  (set `self.onDamage` true)
  (set `self.damage bool` (`KismetMathLibrary.RandomBool`))
  (`PaperFlipbookComponent.SetFlipbook` (`self.Sprite`) (select `bool` (`self.damage bool`) :`false` "/Game/Flipbooks/NinjaSword/SNinja_hurt.SNinja_hurt" :`true` "/Game/Flipbooks/NinjaSword/SNinja_hurt2.SNinja_hurt2" :!type "PaperFlipbook Object Reference"))
  (`KismetSystemLibrary.RetriggerableDelay` (select `bool` (`self.damage bool`) :`false` 0.13 :`true` 0.2 :!type "Float (single-precision)"))
  (set `self.onDamage` false)
  (if (<= (`self.health`) 0.0)
    (set `self.isDead` true)
    (`self.K2_DestroyActor`)))

(fn `Attack`
  (bind (_outhit _returnvalue) (`KismetSystemLibrary.BoxTraceSingle` :`Start` (`self.K2_GetActorLocation`) :`End` (`SceneComponent.K2_GetComponentLocation` (`self.AttackOffest`)) :`HalfSize` (0.0 10.0 32.0) :`TraceChannel` "TraceTypeQuery2" :`DrawDebugType` "ForOneFrame"))
  (if _returnvalue
    (bind (_bblockinghit _binitialoverlap _time _distance _location _impactpoint _normal _impactnormal _physmat _hitactor) (`GameplayStatics.BreakHitResult` _outhit))
    (if (== _hitactor (`GameplayStatics.GetPlayerCharacter` 0))
      (`GameplayStatics.ApplyDamage` _hitactor 1.0 null self))))

(fn `Flip`
  (bind _output_get (set `self.isFacingRight` (not (`self.isFacingRight`))))
  (`SceneComponent.K2_SetRelativeRotation` (`self.Sprite`) (select `bool` _output_get :`false` (struct :`Yaw` 180.0) :!type "Rotator Structure") false false)
  (set `self.distanceToFlip` (`self.initDistanceToFlip`)))

(fn `HasEnemyOnFront`
  (returns (`Return Value` :type Boolean))
  (bind (_outhit _returnvalue) (`KismetSystemLibrary.LineTraceSingle` (`self.K2_GetActorLocation`) (`SceneComponent.K2_GetComponentLocation` (`self.AttackTrace`)) "TraceTypeQuery2"))
  (if _returnvalue
    (return (== (`.HitActor` (`GameplayStatics.BreakHitResult` _outhit)) (`GameplayStatics.GetPlayerCharacter` 0)))
    (else
      (return false))))

(fn `HasGroundOnFront`
  (returns (ReturnValue :type Boolean))
  (bind (_outhit _returnvalue) (`KismetSystemLibrary.LineTraceSingle` (`SceneComponent.K2_GetComponentLocation` (`self.StartFrontTrace`)) (`SceneComponent.K2_GetComponentLocation` (`self.EndFrountGroundTrace`)) "TraceTypeQuery1"))
  (if _returnvalue
    (cast `PaperTileMapActor` (`.HitActor` (`GameplayStatics.BreakHitResult` _outhit))
      (:`then`
        _)
      (:`CastFailed`
        _))
    (return true)
    (else
      (return false))))

(fn `HasObstaclesOnFront`
  (returns (ReturnValue :type Boolean))
  (bind (_outhit _returnvalue) (`KismetSystemLibrary.LineTraceSingle` (`self.K2_GetActorLocation`) (`SceneComponent.K2_GetComponentLocation` (`self.FriendOffest`)) "TraceTypeQuery2"))
  (if _returnvalue
    (bind (_bblockinghit _binitialoverlap _time _distance _location _impactpoint _normal _impactnormal _physmat _hitactor) (`GameplayStatics.BreakHitResult` _outhit))
    (cast `/Game/Blueprints/Character/NinjaSword` _hitactor
      (:`then`
        (return true))
      (:`CastFailed`
        (cast `PaperSpriteActor` _hitactor
          (:`then`
            (return true))
          (:`CastFailed`
            _)))))
  (return false))

(fn `Move`
  (`self.AddMovementInput` (1.0 0.0 0.0) (select `bool` (`self.isFacingRight`) :`false` -1.0 :`true` 1.0 :!type "Float (single-precision)"))
  (`PaperFlipbookComponent.SetFlipbook` (`self.Sprite`) "/Game/Flipbooks/NinjaSword/SNinja_run.SNinja_run")
  (if (`self.isDistanceToFlip`)
    (set `self.distanceToFlip` (- (`self.distanceToFlip`) (`KismetMathLibrary.VSize` (* (`self.GetVelocity`) (`self.deltaTime`)))))))

(fn `UserConstructionScript`
  (bind (_returnvalue_x _returnvalue_y) (`KismetMathLibrary.BreakVector` (`self.K2_GetActorLocation`)))
  (set `self.initY` _returnvalue_y)
  (set `self.initDistanceToFlip` (`self.distanceToFlip`)))